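; BP_Visibility sets the in-game visibility of weapons by type and puts the WBP_UI widget on screen at BeginPlay.
; It loads every row of DT_WeaponsType into the WeaponsType array, then calls FindAllWeaponsByTag.
; That function finds actors by each type's tag, caches them in that array entry and hides or shows them according to its Visible flag.
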(event EventBeginPlay
  (bind _returnvalue (Game|ConstructObjectfromClass "/Game/MAINProject/Blueprints/UI/WBP_UI.WBP_UI_C"))
  (bind _output_get (Variables|Default|SetWBP_UI _returnvalue))
  (UserInterface|Viewport|AddtoViewport _output_get 0)
  (bind _outrownames (DataTable|GetDataTableRowNames "/Game/MAINProject/Blueprints/DT_WeaponsType.DT_WeaponsType"))
  (Variables|Default|SetLoadedWeapons (Utilities|Array|MakeArray ""))
  (for _array_element _outrownames
    (bind _returnvalue_2 (Utilities|GetDataTableRow "/Game/MAINProject/Blueprints/DT_WeaponsType.DT_WeaponsType" _array_element)
      (:then
        (Utilities|Array|Add (Variables|Default|GetLoadedWeapons) _returnvalue_2))))
  (Variables|Default|SetWeaponsType (Variables|Default|GetLoadedWeapons))
  (CallFunction|FindAllWeaponsbyTag))

(fn ConstructionScript)

(fn FindAllWeaponsbyTag
  (for (_array_element _array_index) (Variables|Default|GetWeaponsType)
    (bind _outactors (Actor|GetAllActorswithTag (Utilities|String|StringToName (.Tag (Utilities|Struct|BreakS_WeaponType _array_element)))))
    (Utilities|Array|SetArrayElem (Variables|Default|GetWeaponsType) _array_index (Utilities|Struct|MakeS_WeaponType (.Tag (Utilities|Struct|BreakS_WeaponType _array_element)) (.DisplayName (Utilities|Struct|BreakS_WeaponType _array_element)) _outactors (.Visible (Utilities|Struct|BreakS_WeaponType _array_element))))
    (for _array_element_2 _outactors
      (Rendering|SetActorHiddenInGame _array_element_2 (not (.Visible (Utilities|Struct|BreakS_WeaponType _array_element)))))))